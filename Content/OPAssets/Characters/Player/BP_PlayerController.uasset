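; Player controller that creates the player's HUD on begin play and manages pausing and resuming the game.
; The pause input action either pauses, hiding the HUD and showing a lazily created, reused pause menu with the mouse cursor, or sends the active UINav widget back to its parent if already paused.
; Removal of the root menu widget triggers resuming, which restores the HUD and game-only input and hides the cursor.
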(event `self.ReceiveBeginPlay`
  (bind _returnvalue (`|CreateWidget` "/Game/OPAssets/UserInterface/WBP_HUD.WBP_HUD_C" self))
  (bind _output_get (set `self.PlayerHUD` _returnvalue))
  (`UserWidget.AddToPlayerScreen` _output_get 0))

(event `EnhancedInput|/Game/OPAssets/Input/InputActions/Universal/IA_PauseResumeGame`
  (params (ActionValue :type Boolean) (ElapsedSeconds :type "Float (double-precision)") (TriggeredSeconds :type "Float (double-precision)") (InputAction :type "InputAction Object Reference" :default "/Game/OPAssets/Input/InputActions/Universal/IA_PauseResumeGame.IA_PauseResumeGame"))
  (:`Triggered`
    (if (`GameplayStatics.IsGamePaused`)
      (`UINavWidget.ReturnToParent` (`UINavPCComponent.GetActiveWidget` (`self.UINavPC`)) true 0)
      (else
        (`self.PauseGame`)))))

(event `self.OnRootWidgetRemoved`
  (`self.ResumeGame`))

(fn `PauseGame`
  ;[1 1 1] Hides the player's HUD, shows the pause menu, pauses the game, and shows the mouse cursor.
  (`Widget.SetVisibility` (`self.PlayerHUD`) "Collapsed")
  (`/Engine/EditorBlueprintResources/StandardMacros.IsValid` (`self.PauseMenu`)
    (:`Is Valid`
      _)
    (:`Is Not Valid`
      (bind _returnvalue (`|CreateWidget` "/Game/OPAssets/UserInterface/Menus/UIN_PauseMenu.UIN_PauseMenu_C" self))
      (bind _output_get (set `self.PauseMenu` _returnvalue))))
  (`UserWidget.AddToPlayerScreen` _output_get 0)
  (`WidgetBlueprintLibrary.SetInputMode_GameAndUIEx` self null "DoNotLock" true true)
  (`GameplayStatics.SetGamePaused` true)
  (set `self.bShowMouseCursor` true))

(fn `ResumeGame`
  ;[1 1 1] Shows the player's HUD, unpauses the game, and hides the mouse cursor.
  (`Widget.SetVisibility` (`self.PlayerHUD`) "SelfHitTestInvisible")
  (`OZEFunctionLibrary.CustomGameOnlyInputMode` 0)
  (`GameplayStatics.SetGamePaused` false)
  (set `self.bShowMouseCursor` false))

(fn `UserConstructionScript`)